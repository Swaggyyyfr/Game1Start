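; Stealth-game enemy AI Blueprint that patrols, chases and melee-attacks the player.
; Tick uses CanMove and PlayerVisible flags to select chasing, target-point patrol or random roaming via AIMoveTo, with varying walk speeds.
; PawnSensing handles sight and noise, though sight only ever sets PlayerVisible false, leaving chase untriggered here.
; Attack montage notify sphere-traces from the hand, loading the player's checkpoint on hit; DoOnce resets while Hostile.
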(event OnSeePawn(PawnSensing)
  (params (Pawn :type Pawn%20Object%20Reference))
  (Utilities|FlowControl|Sequence
    (:then_1
      (Utilities|Casting|CastToBP_ThirdPersonCharacterCustom Pawn
        (:then
          (Development|PrintString "HEY! STOP!!!" true true "(R=1.000000,G=0.190411,B=0.001048,A=1.000000)")
          (Variables|Default|SetPlayer%20visible false))
        (:CastFailed
          (Variables|Default|SetPlayer%20visible false))))
    (:then_2
      (Utilities|FlowControl|RetriggerableDelay 3.0)
      (Variables|Default|SetPlayer%20visible false)
      (Development|PrintString "Musta lost my marbles" true true "(R=0.070162,G=0.543403,B=0.413537,A=1.000000)"))))

(event OnHearNoise(PawnSensing)
  (params (Instigator :type Pawn%20Object%20Reference) (Location :type Vector%20%28by%20ref%29 :default "0, 0, 0") (Volume :type Float%20%28single-precision%29))
  (CallFunction|UpdateWalkSpeed 2e+02)
  (Variables|Default|SetCan%20move false)
  (AI|AIMoveTo self "0, 0, 0" 0 5.0 false
    (:OnSuccess
      (Utilities|FlowControl|Delay 12.0)
      (Variables|Default|SetCan%20move true))))

(event Custom|Chase%20Player
  (CallFunction|UpdateWalkSpeed 5e+02)
  (if (Variables|Default|GetPlayer%20visible)
    (Variables|Default|SetCan%20move false)
    (AI|AIMoveTo self "0, 0, 0" (Game|GetPlayerCharacter 0) 5e+01 false
      (:OnSuccess
        (Variables|Default|SetCan%20move true)
        (CallFunction|Attack)
        (Development|PrintString "doink")))))

(event Custom|Attack
  (bind _mesh (Variables|Character|GetMesh))
  (bind _returnvalue (Transformation|GetSocketLocation _mesh "hand_r"))
  ;[0.15 0.1407 0.04319 0.5] Bonk
  (Utilities|FlowControl|DoOnce false ; Only Reset Attack on miss.
    (:Completed
      (bind _notifyname (Animation|Montage|PlayMontage (Variables|Character|GetMesh) "/Game/StealthGame/Characters/Enemies/AM_Attack_01.AM_Attack_01") ; Play the AM_Attack_01
        (:OnCompleted
          (if (Variables|Default|GetbHostile) ; Keep attacking if you haven't landed the hit.
            (CallFunction|ResetAttack)))
        (:OnNotifyBegin
          (switch name _notifyname ; Pick the proper attack type(standard when there is more than one type of attack)
            (:AttackDamage
              (Development|PrintString "I'm attacking!")
              (bind (_outhits _returnvalue_2) (Collision|MultiSphereTraceForObjects _returnvalue (+ _returnvalue (* (Transformation|GetActorForwardVector) (Variables|Default|GetMelee%20Trace%20Distance))) (Variables|Default|GetRadius) (Utilities|Array|MakeArray "ObjectTypeQuery3") false 0 "ForDuration")) ; Trace forward from hand socket.
              (if _returnvalue_2 ; If a pawn is hit in that trace...
                (for _array_element _outhits ; ...loop through the results....
                  (bind _asbp_third_person_character_custom (Utilities|Casting|CastToBP_ThirdPersonCharacterCustom (.HitActor (Collision|BreakHitResult _array_element))))
                  (Default|LoadCheckpoint _asbp_third_person_character_custom)
                  (Variables|Default|SetbHostile false) ; ...and stop attacking...
                )))))))))

(event Custom|Move%20to%20patrol%20point
  (bind _target_points (Variables|Default|GetTarget%20points))
  (bind _patroltargetpoints (Variables|Default|GetPatrolTargetPoints))
  (bind _output (Utilities|Array|Get(acopy) _target_points _patroltargetpoints))
  (CallFunction|UpdateWalkSpeed 3e+02)
  (Variables|Default|SetCan%20move false)
  (Development|PrintString (Utilities|String|ToString(Boolean) (Utilities|IsValid _output)))
  (bind _movementresult (AI|AIMoveTo self "0, 0, 0" _output 5.0 false)
    (:OnSuccess
      (CallFunction|SetNextPatrolPointIndex)
      (Utilities|FlowControl|Delay 1.5)
      (Variables|Default|SetCan%20move true))
    (:OnFail
      (Development|PrintString (Utilities|String|EnumtoString _movementresult)))))

(event Custom|ResetAttack
  (bind _mesh (Variables|Character|GetMesh))
  (bind _returnvalue (Transformation|GetSocketLocation _mesh "hand_r"))
  ;[0.15 0.1407 0.04319 0.5] Bonk
  (Utilities|FlowControl|DoOnce false) ; enters at Reset
)

(event Custom|random%20patrol
  (Rendering|Material|SetMaterial (Variables|Character|GetMesh) 0 "/Game/StealthGame/Core/Characters/PlayerCharacter/Mannequins/Materials/M_Mannequin.M_Mannequin")
  (CallFunction|UpdateWalkSpeed 3e+02)
  (Variables|Default|SetCan%20move false)
  (AI|AIMoveTo self (.RandomLocation (AI|Navigation|GetRandomReachablePointinRadius (Transformation|GetActorLocation) 2e+03 0 0)) 0 75.0 false
    (:OnSuccess
      (Utilities|FlowControl|Delay 1.0)
      (Variables|Default|SetCan%20move true))))

(event Custom|SetNextPatrolPointIndex
  (Variables|Default|SetPatrolTargetPoints (Math|Integer|%(Integer) (+ (Variables|Default|GetPatrolTargetPoints) 1) (Utilities|Array|Length (Variables|Default|GetTarget%20points)))))

(event EventBeginPlay
  (Utilities|FlowControl|Sequence
    (:then_0
      (Actor|GetActorOfClass "/Game/StealthGame/Gadgets/NoiseMakers/BP_DistractionItemPawn.BP_DistractionItemPawn_C"))))

(event Collision|EventActorBeginOverlap
  (params (OtherActor :type Actor%20Object%20Reference)))

(event EventTick
  (params (DeltaSeconds :type Float%20%28single-precision%29))
  (bind _player_visible (Variables|Default|GetPlayer%20visible))
  (if (Variables|Default|GetCan%20move)
    (if _player_visible
      (CallFunction|ChasePlayer)
      (elif (Variables|Default|GetbTargetPointMovement)
        (CallFunction|MovetoPatrolPoint)
        (else
          (CallFunction|RandomPatrol))))
    (elif _player_visible
      (CallFunction|ChasePlayer))))

(fn ConstructionScript)

(fn UpdateWalkSpeed
  (params (Max%20Walk%20Speed :type Float%20%28single-precision%29))
  (Variables|/Script/Engine.CharacterMovementComponent|SetMaxWalkSpeed (Variables|Character|GetCharacterMovement) Max%20Walk%20Speed))