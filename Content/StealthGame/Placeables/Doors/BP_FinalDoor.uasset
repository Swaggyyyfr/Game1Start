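; BP_FinalDoor is a stealth-game door that opens only for a player character holding more than one key.
; Entering its box trigger with enough keys flip-flops a timeline forward or in reverse, swinging the door's yaw through 90 degrees.
; Without enough keys, it creates a master-locked widget and plays its animation.
; Leaving the box only clears an Inside flag, which is never set true and drives nothing.
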(event OnComponentBeginOverlap(Box)
  (params (OverlappedComponent :type Primitive%20Component%20Object%20Reference) (OtherActor :type Actor%20Object%20Reference) (OtherComp :type Primitive%20Component%20Object%20Reference) (OtherBodyIndex :type Integer) (bFromSweep :type Boolean) (SweepResult :type Hit%20Result%20Structure%20%28by%20ref%29))
  (bind _asbp_third_person_character_custom (Utilities|Casting|CastToBP_ThirdPersonCharacterCustom OtherActor))
  (if (> (Variables|/Game/StealthGame/Core/Characters/PlayerCharacter/BP_ThirdPersonCharacterCustom.BP_ThirdPersonCharacterCustom_C|GetKey%20Count _asbp_third_person_character_custom) 1)
    (Development|PrintText "Access Granted")
    (Utilities|FlowControl|FlipFlop
      (:A
        (bind _newtrack_0 (Timeline|Timeline Play)
          (:Update
            (Transformation|SetRelativeRotation (Variables|Default|GetDoor) (Math|Rotator|MakeRotator 0.0 0.0 (* _newtrack_0 -9e+01)) false false))))
      (:B
        (Timeline|Timeline Reverse)))
    (else
      (bind _returnvalue (UserInterface|CreateWidget "/Game/StealthGame/WBP_MasterLockedDoor1.WBP_MasterLockedDoor1_C"))
      (UserInterface|Viewport|AddtoViewport _returnvalue 0)
      (Default|PlayDoorlockedAnimation _returnvalue))))

(event OnComponentEndOverlap(Box)
  (params (OverlappedComponent :type Primitive%20Component%20Object%20Reference) (OtherActor :type Actor%20Object%20Reference) (OtherComp :type Primitive%20Component%20Object%20Reference) (OtherBodyIndex :type Integer))
  (Utilities|Casting|CastToBP_ThirdPersonCharacterCustom OtherActor)
  (Variables|Default|Setinside? false))

(event EventTick
  (params (DeltaSeconds :type Float%20%28single-precision%29))
  (if (Variables|Default|Getinside?)
    _))

(fn ConstructionScript)